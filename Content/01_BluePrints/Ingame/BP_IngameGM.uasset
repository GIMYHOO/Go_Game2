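; In-game Blueprint (GM) that runs the lap and cumulative clear timers, storing values and display text in Bp_GI so they persist across levels.
; Two timelines started on BeginPlay act as clocks: one writes lap time, the other shows saved clear time plus elapsed time.
; set_Gi_time adds the lap to the saved total and resets the clear-time timeline's position.
; Reset_ClearTime clears the stored times for non-stage level changes.
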(event Custom|Reset_ClearTime
  (bind _bp_gi (Variables|Default|GetBP_GI))
  ;[1 1 1] 스테이지 이동이 아닌 레벨이동시 모든 시간 초기화
  (Variables|/Game/01_BluePrints/UsingStuff/Bp_GI.Bp_GI_C|SetLapTime (Variables|Default|GetBP_GI) 0.0)
  (Variables|/Game/01_BluePrints/UsingStuff/Bp_GI.Bp_GI_C|SetClearTime _bp_gi 0.0)
  (Variables|/Game/01_BluePrints/UsingStuff/Bp_GI.Bp_GI_C|SetClearTime_text _bp_gi " "))

(event Custom|Starttime
  ;[1 1 1] 클리어타임 실시간 출력
  (bind _time (Timeline|타임라인_1 Play)
    (:Update
      (Variables|/Game/01_BluePrints/UsingStuff/Bp_GI.Bp_GI_C|SetClearTime_text (Variables|Default|GetBP_GI) (Utilities|TimetoText (+ _time (Variables|/Game/01_BluePrints/UsingStuff/Bp_GI.Bp_GI_C|GetClearTime (Variables|Default|GetBP_GI))))))))

(event Custom|set_Gi_time
  ;[1 1 1] Destroy 이전 시간 저장 후 추가
  (bind _output_get (Variables|/Game/01_BluePrints/UsingStuff/Bp_GI.Bp_GI_C|SetClearTime (Variables|Default|GetBP_GI) (+ (Variables|/Game/01_BluePrints/UsingStuff/Bp_GI.Bp_GI_C|GetClearTime (Variables|Default|GetBP_GI)) (Variables|/Game/01_BluePrints/UsingStuff/Bp_GI.Bp_GI_C|GetLapTime (Variables|Default|GetBP_GI)))))
  (Variables|/Game/01_BluePrints/UsingStuff/Bp_GI.Bp_GI_C|SetClearTime_text (Variables|Default|GetBP_GI) (Utilities|TimetoText _output_get))
  ;[1 1 1] 클리어타임 실시간 출력
  (bind _time (Timeline|타임라인_1 SetNewTime)
    (:Update
      (Variables|/Game/01_BluePrints/UsingStuff/Bp_GI.Bp_GI_C|SetClearTime_text (Variables|Default|GetBP_GI) (Utilities|TimetoText (+ _time (Variables|/Game/01_BluePrints/UsingStuff/Bp_GI.Bp_GI_C|GetClearTime (Variables|Default|GetBP_GI))))))))

(event Custom|StartLaptime
  ;[1 1 1] LapTime
  (bind _time (Timeline|타임라인_0 Play)
    (:Update
      (bind _output_get (Variables|/Game/01_BluePrints/UsingStuff/Bp_GI.Bp_GI_C|SetLapTime (Variables|Default|GetBP_GI) _time))
      (Variables|/Game/01_BluePrints/UsingStuff/Bp_GI.Bp_GI_C|Setlaptiem_text (Variables|Default|GetBP_GI) (Utilities|TimetoText _output_get)))))

(event EventBeginPlay
  (CallFunction|Starttime)
  (CallFunction|StartLaptime)
  (bind _asbp_gi (Utilities|Casting|CastToBp_GI (Game|GetGameInstance)))
  (Variables|Default|SetBP_GI _asbp_gi))

(fn ConstructionScript)