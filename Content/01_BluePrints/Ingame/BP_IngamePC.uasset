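; BP_IngamePC is an in-game Blueprint that shows the lap time and clear time on a HUD.
; On BeginPlay it creates the UMG_IngameWidget and adds it to the viewport.
; Each Tick it casts the game instance to Bp_GI and copies its lap and clear time texts into the widget's text fields.
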(event EventTick
  (params (DeltaSeconds :type Float%20%28single-precision%29))
  (bind _asbp_gi (Utilities|Casting|CastToBp_GI (Game|GetGameInstance)))
  (Rendering|Components|TextRender|SetText (Variables|/Game/01_BluePrints/Ingame/UMG_IngameWidget.UMG_IngameWidget_C|GetLapTimeSet (Variables|Default|GetUMG_Ingamewidget)) (Variables|/Game/01_BluePrints/UsingStuff/Bp_GI.Bp_GI_C|Getlaptiem_text _asbp_gi))
  (Rendering|Components|TextRender|SetText (Variables|/Game/01_BluePrints/Ingame/UMG_IngameWidget.UMG_IngameWidget_C|GetClearTimeset (Variables|Default|GetUMG_Ingamewidget)) (Variables|/Game/01_BluePrints/UsingStuff/Bp_GI.Bp_GI_C|GetClearTime_text _asbp_gi)))

(event EventBeginPlay
  (bind _returnvalue (UserInterface|CreateWidget "/Game/01_BluePrints/Ingame/UMG_IngameWidget.UMG_IngameWidget_C"))
  (bind _output_get (Variables|Default|SetUMG_Ingamewidget _returnvalue))
  (UserInterface|Viewport|AddtoViewport _output_get 0))

(fn ConstructionScript)