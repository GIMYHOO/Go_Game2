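; BP_Trap_Bullet_2 is a short-lived trap projectile that reacts when it hits a BP_Charater and expires after a few seconds otherwise.
; Its Box overlap filters for that character class, then plays an attached sound, spawns a scaled-down fire impact emitter, prints an arrow-death debug message and destroys the actor.
; The graphs apply no damage themselves, and a separate DestroyRocket function only destroys the actor.
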(event OnComponentBeginOverlap(Box)
  (params (OverlappedComponent :type Primitive%20Component%20Object%20Reference) (OtherActor :type Actor%20Object%20Reference) (OtherComp :type Primitive%20Component%20Object%20Reference) (OtherBodyIndex :type Integer) (bFromSweep :type Boolean) (SweepResult :type Hit%20Result%20Structure%20%28by%20ref%29))
  (Utilities|Casting|CastToBP_Charater OtherActor)
  (Audio|SpawnSoundAttached 0 (Variables|Default|GetBox))
  (Effects|SpawnEmitteratLocation "/Game/04_eff/04eff_Impact_Player_Fire_Strong.04eff_Impact_Player_Fire_Strong" (Transformation|GetActorLocation) (Transformation|GetActorRotation) "0.500000,0.500000,0.500000")
  (Development|PrintString "daed : Reason to Arrow")
  (Actor|DestroyActor))

(event EventBeginPlay
  (Actor|SetLifeSpan 3.0))

(fn ConstructionScript)

(fn DestroyRocket
  (Actor|DestroyActor))