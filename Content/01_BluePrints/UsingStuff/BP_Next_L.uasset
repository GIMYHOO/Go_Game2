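; Level-exit trigger Blueprint that moves play to the next map in a nine-entry sequence when anything overlaps its Box.
; It finds the current level name in NextLevleArray, then prints and opens the following entry, or opens Lobby after the last one.
; A preliminary check against NextLevle gates the search loop; when the names match, execution skips straight to the comparison without iterating.
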(event OnComponentBeginOverlap(Box)
  (params (OverlappedComponent :type Primitive%20Component%20Object%20Reference) (OtherActor :type Actor%20Object%20Reference) (OtherComp :type Primitive%20Component%20Object%20Reference) (OtherBodyIndex :type Integer) (bFromSweep :type Boolean) (SweepResult :type Hit%20Result%20Structure%20%28by%20ref%29))
  (bind _nextlevle_array (Variables|Default|GetNextLevle_array))
  (bind _returnvalue (Game|GetCurrentLevelName true))
  (if (Utilities|Name|NotEqual(Name) (Variables|Default|GetNextLevle) (Utilities|String|StringToName _returnvalue))
    (for _index (range 0 8)
      (bind _output_get (Variables|Default|Setindex _index))
      (bind _returnvalue_2 (Game|GetCurrentLevelName true))
      (if (Utilities|Enum|Equal(Enum) (Utilities|String|ToString(Name) (Utilities|Array|Get(acopy) _nextlevle_array _output_get)) _returnvalue_2)
        (if (== (Variables|Default|Getindex) 8)
          (Game|OpenLevel(byName) "Lobby")
          (else
            (Development|PrintString (Utilities|String|ToString(Name) (Utilities|Array|Get(acopy) _nextlevle_array (+ (Variables|Default|Getindex) 1))))
            (bind _output_get_2 (Variables|Default|SetNextLevle_0 (Utilities|Array|Get(acopy) _nextlevle_array (+ (Variables|Default|Getindex) 1))))
            (Game|OpenLevel(byName) _output_get_2 true "World'/Game/02_Map/SingleMaps'")))))
    (if (Utilities|Enum|Equal(Enum) (Utilities|String|ToString(Name) (Utilities|Array|Get(acopy) _nextlevle_array _output_get)) _returnvalue_2)
      (if (== (Variables|Default|Getindex) 8)
        (Game|OpenLevel(byName) "Lobby")
        (else
          (Development|PrintString (Utilities|String|ToString(Name) (Utilities|Array|Get(acopy) _nextlevle_array (+ (Variables|Default|Getindex) 1))))
          (bind _output_get_3 (Variables|Default|SetNextLevle_0 (Utilities|Array|Get(acopy) _nextlevle_array (+ (Variables|Default|Getindex) 1))))
          (Game|OpenLevel(byName) _output_get_3 true "World'/Game/02_Map/SingleMaps'"))))))

(fn ConstructionScript)