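; BP_PushSwitch is an overlap-triggered switch that notifies linked objects when it is pressed or released.
; Box overlap begin and end toggle a material scalar on the static mesh and send switch or release messages to every entry in Item.
; IsPushed is set inversely to its name: false on begin overlap, true on end overlap.
; NewFunction0 creates a dynamic material instance but is not called in these graphs.
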(event OnComponentBeginOverlap(Box)
  (params (OverlappedComponent :type Primitive%20Component%20Object%20Reference) (OtherActor :type Actor%20Object%20Reference) (OtherComp :type Primitive%20Component%20Object%20Reference) (OtherBodyIndex :type Integer) (bFromSweep :type Boolean) (SweepResult :type Hit%20Result%20Structure%20%28by%20ref%29))
  (Variables|Default|SetIs_pushed? false)
  (Rendering|Material|SetScalarParameterValueonMaterials (Variables|Default|GetStaticMesh) "active_parameter_1" 1.0)
  (for _array_element (Variables|Default|Getitem)
    (Class|BPIItem|Onswitch(Message) _array_element)))

(event OnComponentEndOverlap(Box)
  (params (OverlappedComponent :type Primitive%20Component%20Object%20Reference) (OtherActor :type Actor%20Object%20Reference) (OtherComp :type Primitive%20Component%20Object%20Reference) (OtherBodyIndex :type Integer))
  (Variables|Default|SetIs_pushed? true)
  (Rendering|Material|SetScalarParameterValueonMaterials (Variables|Default|GetStaticMesh) "active_parameter_1" 0.0)
  (for _array_element (Variables|Default|Getitem)
    (Class|BPIItem|OnRelesed(Message) _array_element)))

(fn ConstructionScript)

(fn NewFunction0
  (bind _returnvalue (Rendering|Material|CreateDynamicMaterialInstance (Variables|Default|GetStaticMesh) 0 0 :!class /Script/Engine.PrimitiveComponent))
  (Variables|Default|SetisOn _returnvalue))

(fn GetBindingName
  (return "None"))

(fn GetCurves
  (return 0))

(fn GetCurveValue
  (params (CurveName :type Name :default "None"))
  (return 0.0))