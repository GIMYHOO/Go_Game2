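; BP_TimerSwitch is a timed switch that changes its material and notifies linked actors in the Item array.
; At BeginPlay, an unpushed switch creates a dynamic material and starts the Colortimer timeline, whose updates play Functime.
; Functime updates apply Colortimer's color and set Ispushed only while its track equals exactly 7.
; Box overlap stops Colortimer, then uses Ispushed to set green or red and send switch or release messages.
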(event OnComponentBeginOverlap(Box)
  (params (OverlappedComponent :type Primitive%20Component%20Object%20Reference) (OtherActor :type Actor%20Object%20Reference) (OtherComp :type Primitive%20Component%20Object%20Reference) (OtherBodyIndex :type Integer) (bFromSweep :type Boolean) (SweepResult :type Hit%20Result%20Structure%20%28by%20ref%29))
  (bind _my_material (Variables|Default|GetMy_material))
  (CallFunction|Stopcolor)
  (if (Variables|Default|Getispushed)
    (Variables|Default|Setispushed true)
    (Rendering|Material|SetVectorParameterValue _my_material "DefaultColor" "(R=0.000000,G=1.000000,B=0.290000,A=1.000000)" :!class /Script/Engine.MaterialInstanceDynamic)
    (Rendering|Material|SetScalarParameterValue (Variables|Default|GetMy_material) "active_parameter_2" 4.5e+02 :!class /Script/Engine.MaterialInstanceDynamic)
    (for _array_element (Variables|Default|Getitem)
      (Class|BPIItem|Onswitch(Message) _array_element))
    (else
      (Variables|Default|Setispushed false)
      (Rendering|Material|SetVectorParameterValue _my_material "DefaultColor" "(R=1.000000,G=0.000000,B=0.000000,A=1.000000)" :!class /Script/Engine.MaterialInstanceDynamic)
      (Rendering|Material|SetScalarParameterValue _my_material "active_parameter_2" 0.0 :!class /Script/Engine.MaterialInstanceDynamic)
      (for _array_element_2 (Variables|Default|Getitem)
        (Class|BPIItem|OnRelesed(Message) _array_element_2)))))

(event Custom|Stopcolor
  (Rendering|Material|SetVectorParameterValue (Variables|Default|GetMy_material) "DefaultColor" "(R=0.000000,G=1.000000,B=0.290000,A=1.000000)" :!class /Script/Engine.MaterialInstanceDynamic)
  (bind _새_트랙_2 (Timeline|colortimer Stop)
    (:Update
      (bind _새_트랙_4 (Timeline|functime Play)
        (:Update
          (Rendering|Material|SetVectorParameterValue (stale Custom|begintimer _output_get) "DefaultColor" _새_트랙_2 :!class /Script/Engine.MaterialInstanceDynamic)
          (if (== _새_트랙_4 7.0)
            (Rendering|Material|SetScalarParameterValue (Variables|Default|GetMy_material) "active_parameter_2" 4.5e+02 :!class /Script/Engine.MaterialInstanceDynamic))
          (if (== _새_트랙_4 7.0)
            (Variables|Default|Setispushed true)
            (else
              (Variables|Default|Setispushed false))))))))

(event Custom|begintimer
  (bind _returnvalue (Rendering|Material|CreateDynamicMaterialInstance (Variables|Default|GetStaticMesh) 0 0 :!class /Script/Engine.PrimitiveComponent))
  (bind _output_get (Variables|Default|SetMy_material _returnvalue))
  (bind _새_트랙_2 (Timeline|colortimer Play)
    (:Update
      (bind _새_트랙_4 (Timeline|functime Play)
        (:Update
          (Rendering|Material|SetVectorParameterValue _output_get "DefaultColor" _새_트랙_2 :!class /Script/Engine.MaterialInstanceDynamic)
          (if (== _새_트랙_4 7.0)
            (Rendering|Material|SetScalarParameterValue (Variables|Default|GetMy_material) "active_parameter_2" 4.5e+02 :!class /Script/Engine.MaterialInstanceDynamic))
          (if (== _새_트랙_4 7.0)
            (Variables|Default|Setispushed true)
            (else
              (Variables|Default|Setispushed false))))))))

(event Custom|Switch_on
  (if (Variables|Default|Getispushed)
    (for _array_element (Variables|Default|Getitem)
      (Class|BPIItem|Onswitch(Message) _array_element))
    (else
      (for _array_element_2 (Variables|Default|Getitem)
        (Class|BPIItem|OnRelesed(Message) _array_element_2)))))

(event EventBeginPlay
  ;[1 1 1] begin
  (if (not (Variables|Default|Getispushed))
    (CallFunction|Begintimer)))

(fn ConstructionScript)